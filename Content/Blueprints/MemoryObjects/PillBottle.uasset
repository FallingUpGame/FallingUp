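; Pill bottle memory object, a child Blueprint that supplies its own voice clip and highlight materials to shared parent logic.
; Its construction script runs the parent's, then sets the Kay apology audio, the normal bottle material and a white board material for glowing.
; Glow and Unglow call the parent versions, passing the bottle, the matching material and the material slot to change.
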(event EventBeginPlay)

(event Collision|EventActorBeginOverlap
  (params (OtherActor :type Actor%20Object%20Reference)))

(event EventTick
  (params (DeltaSeconds :type Float%20%28single-precision%29)))

(event EventGlow
  (params (Object :type Static%20Mesh%20Component%20Object%20Reference) (Material :type Material%20Object%20Reference) (Element :type Integer))
  (|CallParentFunction (Variables|Default|GetPillBottle) (Variables|Default|GetMaterial_2) 1))

(event EventUnglow
  (params (Object :type Static%20Mesh%20Component%20Object%20Reference) (Material :type Material%20Object%20Reference) (Element :type Integer))
  (|CallParentFunction (Variables|Default|GetPillBottle) (Variables|Default|GetMaterial) 1))

(fn ConstructionScript
  (|CallParentFunction)
  (Variables|Default|SetAudio "/Game/Audio/Kay_I_m_Sorry_Wave.Kay_I_m_Sorry_Wave")
  (Variables|Default|SetMaterial "/Game/Materials/M_PillBottle.M_PillBottle")
  (Variables|Default|SetMaterial_2 "/Game/Materials/M_Board_White.M_Board_White"))