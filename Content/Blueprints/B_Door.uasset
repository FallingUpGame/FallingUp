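; Interactive door actor that the player opens and closes by touch release or the E key while inside its Box trigger.
; Box overlap enables or disables input on the door and sets LookedAt, which gates touch.
; BeginPlay derives DoorStatus from the starting yaw; each toggle flips it and plays or reverses the DoorRot timeline, which drives relative yaw.
; A check for player movement exists but is disconnected.
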(event OnComponentBeginOverlap(Box)
  (params (OverlappedComponent :type Primitive%20Component%20Object%20Reference) (OtherActor :type Actor%20Object%20Reference) (OtherComp :type Primitive%20Component%20Object%20Reference) (OtherBodyIndex :type Integer) (bFromSweep :type Boolean) (SweepResult :type Hit%20Result%20Structure%20%28by%20ref%29))
  (Input|EnableInput (Game|GetPlayerController 0))
  (Variables|Default|SetLookedAt true))

(event OnComponentEndOverlap(Box)
  (params (OverlappedComponent :type Primitive%20Component%20Object%20Reference) (OtherActor :type Actor%20Object%20Reference) (OtherComp :type Primitive%20Component%20Object%20Reference) (OtherBodyIndex :type Integer))
  (Input|DisableInput (Game|GetPlayerController 0))
  (Variables|Default|SetLookedAt false))

(event EventBeginPlay
  (Variables|Default|SetDoorStatus (> (.Yaw (Math|Rotator|BreakRotator (Transformation|GetActorRotation))) 7e+01)))

(event Collision|EventActorBeginOverlap
  (params (OtherActor :type Actor%20Object%20Reference)))

(event EventTick
  (params (DeltaSeconds :type Float%20%28single-precision%29)))

(event Input|KeyboardEvents|E
  (params (Key :type Key%20Structure :default "AnyKey"))
  (:Pressed
    (if (Variables|Default|GetDoorStatus)
      (Variables|Default|SetDoorStatus false)
      (bind _doorbackrot (Timeline|DoorRot Play)
        (:Update
          (Transformation|SetActorRelativeRotation (Math|Rotator|MakeRotator 0.0 0.0 (- 0.0 _doorbackrot)))))
      (else
        (Variables|Default|SetDoorStatus true)
        (Timeline|DoorRot Reverse)))))

(event Input|TouchEvents|InputTouch
  (params (Location :type Vector) (FingerIndex :type ETouchIndex%20Enum))
  ;[1 1 1] If there is touch input and the player is not moving, open or close the door
  (:Released
    (if (Variables|Default|GetLookedAt)
      (if (Variables|Default|GetDoorStatus)
        (Variables|Default|SetDoorStatus false)
        (bind _doorbackrot (Timeline|DoorRot Play)
          (:Update
            (Transformation|SetActorRelativeRotation (Math|Rotator|MakeRotator 0.0 0.0 (- 0.0 _doorbackrot)))))
        (else
          (Variables|Default|SetDoorStatus true)
          (Timeline|DoorRot Reverse))))))

(fn ConstructionScript)